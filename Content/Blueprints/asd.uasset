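; Breakable statue actor that swaps its static mesh for a Chaos Geometry Collection when struck hard.
; The first hit above an impulse threshold hides the mesh, stops its physics, assigns the fractured statue collection and applies external strain at the impact point.
; Break events move each broken piece to the Debris collision profile and disable the static mesh's collision.
; Radial impulse and walkable slope override nodes are unconnected.
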(event `self.ReceiveHit`
  (params (MyComp :type "PrimitiveComponent Object Reference") (Other :type "Actor Object Reference") (OtherComp :type "PrimitiveComponent Object Reference") (bSelfMoved :type Boolean) (HitLocation :type "Vector Structure") (HitNormal :type "Vector Structure") (NormalImpulse :type "Vector Structure") (Hit :type "HitResult Structure (by ref)"))
  (if (> (`KismetMathLibrary.VSize` NormalImpulse) 10000.0)
    (`/Engine/EditorBlueprintResources/StandardMacros.DoOnce` false
      (:`Completed`
        (`|ExecutionSequence`
          (:`then_0`
            (`SceneComponent.SetVisibility` (`self.StaticMesh`) false false)
            (`PrimitiveComponent.SetSimulatePhysics` (`self.StaticMesh`) false)
            (`GeometryCollectionComponent.SetRestCollection` (`self.GeometryCollection`) "/Game/Blueprints/GC_SM_Statue.GC_SM_Statue" true))
          (:`then_1`
            (`GeometryCollectionComponent.ApplyExternalStrain` (`self.GeometryCollection`) 0 HitLocation 100.0 1 1.0 5000000.0)))))))

(event `self.GeometryCollection.OnChaosBreakEvent`
  (params (BreakEvent :type "ChaosBreakEvent Structure (by ref)"))
  (`GeometryCollectionComponent.SetPerParticleCollisionProfileName` (`self.GeometryCollection`) (`|MakeArray` BreakEvent_Index) "Debris")
  (`PrimitiveComponent.SetCollisionEnabled` (`self.StaticMesh`) "NoCollision"))

(fn `UserConstructionScript`)